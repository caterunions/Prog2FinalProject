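; Game mode for a Spider-Man pizza-collecting time trial, managing the HUD, run timer, pizza count and music.
; A gate on Tick updates run time between timer start and end, and the end shows win stats.
; Death dims the music, then after a delay respawns the player at the start transform and re-enables all pizzas.
; Nested FlipFlops rotate four themed tracks, announced on the HUD.
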(event `OnDeath`
  ; On Player Death
  (`/Game/Blueprints/UI/WBP_HUD.PlayPainAnim` (`self.HUD`))
  (`AudioComponent.AdjustVolume` (`self.CurrentMusic`) 0.0 0.5 "Linear")
  (`KismetSystemLibrary.Delay` 3.0)
  (`self.Reset`))

(event `self.ReceiveBeginPlay`
  ; Player Setup
  (bind _asbp_spiderman (cast `/Game/Blueprints/BP_Spiderman` (`GameplayStatics.GetPlayerPawn` 0)))
  (bind _output_get (set `self.Player` _asbp_spiderman))
  (set `self.PlayerStart` (`self.GetTransform` _output_get))
  ; HUD
  (bind _returnvalue (`|CreateWidget` "/Game/Blueprints/UI/WBP_HUD.WBP_HUD_C"))
  (set `self.HUD` _returnvalue)
  (`UserWidget.AddToViewport` _returnvalue 0)
  (add `/Game/Blueprints/BP_Spiderman.OnDeath` _output_get (delegate `OnDeath`))
  ; Setup Run Variables
  (set `self.RunTime` 0.0)
  (set `self.PizzasCollected` 0)
  (bind _outactors (`GameplayStatics.GetAllActorsOfClass` "/Game/Blueprints/BP_PizzaCollectable.BP_PizzaCollectable_C"))
  (set `self.TotalPizzas` (`KismetArrayLibrary.Array_Length` _outactors)))

(event `self.ReceiveTick`
  (params (DeltaSeconds :type "Float (single-precision)"))
  ; Handle Timer
  (`/Engine/EditorBlueprintResources/StandardMacros.Gate` true :!label _label
    (:`Exit`
      (set `self.RunTime` (- (`KismetSystemLibrary.GetGameTimeInSeconds`) (`self.StartTime`))))))

(event `PizzaCollected`
  ; Pizza Collected
  (`/Engine/EditorBlueprintResources/StandardMacros.IncrementInt` (`self.PizzasCollected`)))

(event `Reset`
  ; Respawn Player
  (`|ExecutionSequence`
    (:`then_0`
      (set `self.RunTime` 0.0)
      (`self.K2_DestroyActor` (`self.Player`))
      (bind _returnvalue (`|SpawnActorFromClass` "/Game/Blueprints/BP_Spiderman.BP_Spiderman_C" (`self.PlayerStart`) "AlwaysSpawn" "MultiplyWithRoot" null null))
      (bind _output_get (set `self.Player` _returnvalue))
      (add `/Game/Blueprints/BP_Spiderman.OnDeath` _output_get (`|CreateDelegate` :!event `OnDeath`))
      (`Controller.Possess` (`GameplayStatics.GetPlayerController` 0) _output_get)
      (goto _label :!via `Close`))
    (:`then_1`
      (set `self.PizzasCollected` 0)
      (bind _outactors (`GameplayStatics.GetAllActorsOfClass` "/Game/Blueprints/BP_PizzaCollectable.BP_PizzaCollectable_C"))
      (for _array_element _outactors
        (`/Game/Blueprints/BP_PizzaCollectable.Enable` _array_element)
        (`AudioComponent.AdjustVolume` (`self.CurrentMusic`) 1.5 1.0 "Linear")
        (`/Game/Blueprints/UI/WBP_HUD.HideWinStats` (`self.HUD`))))))

(event `StartTimer`
  ; Handle Timer
  (set `self.StartTime` (`KismetSystemLibrary.GetGameTimeInSeconds`))
  (`|ExecutionSequence`
    (:`then_0`
      (goto _label :!via `Open`))
    (:`then_1`
      (if (not (`self.MusicPlaying`))
        (`self.CycleMusic`)))))

(event `CycleMusic`
  (bind _currentmusic (`self.CurrentMusic`))
  ; Cycle Music
  (`/Engine/EditorBlueprintResources/StandardMacros.IsValid` _currentmusic
    (:`Is Valid`
      (`AudioComponent.Stop` _currentmusic)
      (`ActorComponent.K2_DestroyComponent` _currentmusic))
    (:`Is Not Valid`
      _))
  (set `self.MusicPlaying` true)
  (`/Engine/EditorBlueprintResources/StandardMacros.FlipFlop`
    (:`A`
      (`/Engine/EditorBlueprintResources/StandardMacros.FlipFlop`
        (:`A`
          (set `self.ChosenMusicFile` "/Game/Audio/Raw/spiderman_ps1_theme.spiderman_ps1_theme")
          (`/Game/Blueprints/UI/WBP_HUD.SetNowPlaying` (`self.HUD`) "Spider-Man PS1 - Theme Song"))
        (:`B`
          (set `self.ChosenMusicFile` "/Game/Audio/Raw/spiderman_3_black_suit_theme.spiderman_3_black_suit_theme")
          (`/Game/Blueprints/UI/WBP_HUD.SetNowPlaying` (`self.HUD`) "Spider-Man 3 - Black Suit Theme"))))
    (:`B`
      (`/Engine/EditorBlueprintResources/StandardMacros.FlipFlop`
        (:`A`
          (set `self.ChosenMusicFile` "/Game/Audio/Raw/spiderman_pizza_theme.spiderman_pizza_theme")
          (`/Game/Blueprints/UI/WBP_HUD.SetNowPlaying` (`self.HUD`) "Spider-Man 2: The Game Pizza Theme"))
        (:`B`
          (set `self.ChosenMusicFile` "/Game/Audio/Raw/whats_up_danger.whats_up_danger")
          (`/Game/Blueprints/UI/WBP_HUD.SetNowPlaying` (`self.HUD`) "Spider-Man: Into the Spider-Verse - What's Up Danger")))))
  (bind _returnvalue (`GameplayStatics.SpawnSound2D` (`self.ChosenMusicFile`) 1.0 1.0 0.0 null false false))
  (set `self.CurrentMusic` _returnvalue))

(event `EndTImer`
  ; Handle Timer
  (`|ExecutionSequence`
    (:`then_0`
      (goto _label :!via `Close`))
    (:`then_1`
      (`/Game/Blueprints/UI/WBP_HUD.ShowWinStats` (`self.HUD`)))))

(fn `UserConstructionScript`)