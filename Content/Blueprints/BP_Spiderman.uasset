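; Player character Blueprint for Spider-Man-style traversal, with camera-relative movement, web grappling and a double jump.
; Grapple input sphere-traces along the camera's forward vector to set an anchor, shown by a stretched DebugWeb arrow.
; Each tick adds pull toward the anchor and, when airborne, projects away-moving velocity onto the tether's tangent plane for swinging.
; A DoOnce-gated air jump redirects horizontal momentum toward input, resetting after ground jumps and grapple release.
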(event `self.ReceiveBeginPlay`
  ; BeginPlay
  (bind _asplayer_controller (cast `PlayerController` (`self.GetController`)))
  (bind _returnvalue (pcsubsystem `EnhancedInputLocalPlayerSubsystem` _asplayer_controller))
  (`EnhancedInputSubsystemInterface.AddMappingContext` _returnvalue "/Game/Input/IMC_CameraMovement.IMC_CameraMovement" 0 (struct))
  (`EnhancedInputSubsystemInterface.AddMappingContext` _returnvalue "/Game/Input/IMC_Movement.IMC_Movement" 0 (struct))
  (`EnhancedInputSubsystemInterface.AddMappingContext` _returnvalue "/Game/Input/IMC_Grapple.IMC_Grapple" 0 (struct))
  (set `self.JumpMaxCount` 2))

(event `self.ReceiveTick`
  (params (DeltaSeconds :type "Float (single-precision)"))
  ; EventTick
  (`self.UpdateGrappleMovement`))

(event `EnhancedInput|/Game/Input/InputActions/IA_Grapple`
  (params (ActionValue :type Boolean) (ElapsedSeconds :type "Float (double-precision)") (TriggeredSeconds :type "Float (double-precision)") (InputAction :type "InputAction Object Reference" :default "/Game/Input/InputActions/IA_Grapple.IA_Grapple"))
  (bind (_returnvalue_x _returnvalue_y _returnvalue_z) (`KismetMathLibrary.BreakVector` (`self.K2_GetActorLocation` self)))
  (bind _returnvalue (`KismetMathLibrary.MakeVector` _returnvalue_x _returnvalue_y (+ _returnvalue_z 70.0)))
  ; Grapple
  (:`Started`
    (bind (_outhit _returnvalue_2) (`KismetSystemLibrary.SphereTraceSingle` _returnvalue (+ _returnvalue (* (`SceneComponent.GetForwardVector` (`self.Camera`)) (`self.GrappleReach`))) 100.0 "TraceTypeQuery1" false (`|MakeArray` self) "None" true (struct :`R` 1.0 :`A` 1.0) (struct :`G` 1.0 :`A` 1.0) 1.0))
    (if _returnvalue_2
      (set `self.GrappleLocation` (`.ImpactPoint` (`GameplayStatics.BreakHitResult` _outhit)))
      (set `self.GrappleAttached` true)))
  (:`Completed`
    (set `self.GrappleAttached` false)
    (`SceneComponent.SetVisibility` (`self.DebugWeb`) false false)
    (`self.RefreshDoubleJump`)))

(event `EnhancedInput|/Game/Input/InputActions/IA_LookRightLeftAxis`
  (params (ActionValue :type "Float (double-precision)") (ElapsedSeconds :type "Float (double-precision)") (TriggeredSeconds :type "Float (double-precision)") (InputAction :type "InputAction Object Reference" :default "/Game/Input/InputActions/IA_LookRightLeftAxis.IA_LookRightLeftAxis"))
  ; Camera Controls
  (:`Triggered`
    (`SceneComponent.K2_AddRelativeRotation` (`self.CameraArm`) (`KismetMathLibrary.MakeRotator` 0.0 0.0 (* ActionValue 3.0)) false false)))

(event `EnhancedInput|/Game/Input/InputActions/IA_MoveForwardBackAxis`
  (params (ActionValue :type "Float (double-precision)") (ElapsedSeconds :type "Float (double-precision)") (TriggeredSeconds :type "Float (double-precision)") (InputAction :type "InputAction Object Reference" :default "/Game/Input/InputActions/IA_MoveForwardBackAxis.IA_MoveForwardBackAxis"))
  (bind (_returnvalue_x _returnvalue_y) (`KismetMathLibrary.BreakVector` (`KismetMathLibrary.GetForwardVector` (`SceneComponent.K2_GetComponentRotation` (`self.Camera`)))))
  ; Movement
  (:`Triggered`
    (`self.AddMovementInput` (`KismetMathLibrary.Normal` (`KismetMathLibrary.MakeVector` _returnvalue_x _returnvalue_y)) ActionValue)))

(event `EnhancedInput|/Game/Input/InputActions/IA_LookUpDownAxis`
  (params (ActionValue :type "Float (double-precision)") (ElapsedSeconds :type "Float (double-precision)") (TriggeredSeconds :type "Float (double-precision)") (InputAction :type "InputAction Object Reference" :default "/Game/Input/InputActions/IA_LookUpDownAxis.IA_LookUpDownAxis"))
  ; Camera Controls
  (:`Triggered`
    (`SceneComponent.K2_AddRelativeRotation` (`self.CameraArm`) (`KismetMathLibrary.MakeRotator` 0.0 (* ActionValue 3.0)) false false)))

(event `EnhancedInput|/Game/Input/InputActions/IA_Jump`
  (params (ActionValue :type Boolean) (ElapsedSeconds :type "Float (double-precision)") (TriggeredSeconds :type "Float (double-precision)") (InputAction :type "InputAction Object Reference" :default "/Game/Input/InputActions/IA_Jump.IA_Jump"))
  (bind (_returnvalue_x _returnvalue_y) (`KismetMathLibrary.BreakVector` (`self.GetLastMovementInputVector`)))
  (bind _charactermovement (`self.CharacterMovement`))
  (bind (_returnvalue_x_2 _returnvalue_y_2) (`KismetMathLibrary.BreakVector` (* (`KismetMathLibrary.VSizeXY` (`MovementComponent.Velocity` _charactermovement)) (`KismetMathLibrary.MakeVector` _returnvalue_x _returnvalue_y))))
  ; Jump + Double Jump
  (:`Started`
    (if (`NavMovementComponent.IsMovingOnGround` (`self.CharacterMovement`))
      (set `self.IsJumping` true)
      (`KismetSystemLibrary.Delay` 0.1)
      (`self.Jump`)
      (`KismetSystemLibrary.Delay` 0.2)
      (set `self.IsJumping` false)
      (`self.RefreshDoubleJump`)
      (else
        (`/Engine/EditorBlueprintResources/StandardMacros.DoOnce` false :!label _label
          (:`Completed`
            (set `self.IsDoubleJumping` true)
            (set `MovementComponent.Velocity` (`KismetMathLibrary.MakeVector` _returnvalue_x_2 _returnvalue_y_2) _charactermovement)
            (`ActorComponent.Activate` (`self.NS_DoubleJump`) true)
            (`self.Jump`)
            (`KismetSystemLibrary.Delay` 0.4)
            (set `self.IsDoubleJumping` false)))))))

(event `EnhancedInput|/Game/Input/InputActions/IA_MoveLeftRightAxis`
  (params (ActionValue :type "Float (double-precision)") (ElapsedSeconds :type "Float (double-precision)") (TriggeredSeconds :type "Float (double-precision)") (InputAction :type "InputAction Object Reference" :default "/Game/Input/InputActions/IA_MoveLeftRightAxis.IA_MoveLeftRightAxis"))
  (bind (_returnvalue_x _returnvalue_y) (`KismetMathLibrary.BreakVector` (`KismetMathLibrary.GetRightVector` (`SceneComponent.K2_GetComponentRotation` (`self.Camera`)))))
  ; Movement
  (:`Triggered`
    (`self.AddMovementInput` (`KismetMathLibrary.Normal` (`KismetMathLibrary.MakeVector` _returnvalue_x _returnvalue_y)) ActionValue)))

(event `RefreshDoubleJump`
  ; Jump + Double Jump
  (goto _label :!via `Reset`))

(fn `UpdateGrappleMovement`
  (bind _returnvalue (`self.K2_GetActorLocation`))
  (bind _charactermovement (`self.CharacterMovement`))
  (bind _debugweb (`self.DebugWeb`))
  (bind _grapplelocation (`self.GrappleLocation`))
  (bind _returnvalue_2 (`KismetMathLibrary.FindLookAtRotation` _returnvalue _grapplelocation))
  (bind _velocity (`MovementComponent.Velocity` _charactermovement))
  (bind _returnvalue_3 (- (`SceneComponent.K2_GetComponentLocation` (`self.CapsuleComponent`)) (`self.GrappleLocation`)))
  (if (`self.GrappleAttached`)
    (`SceneComponent.SetVisibility` (`self.DebugWeb`) true false)
    (set `ArrowComponent.ArrowLength` (`KismetMathLibrary.Vector_Distance` _returnvalue _grapplelocation) _debugweb)
    (`SceneComponent.K2_SetWorldRotation` _debugweb _returnvalue_2 false false)
    (set `MovementComponent.Velocity` (+ (* (`KismetMathLibrary.GetForwardVector` _returnvalue_2) (`self.GrapplePullStrength`)) (`MovementComponent.Velocity` (`self.CharacterMovement`))) (`self.CharacterMovement`))
    (if (and (>= (`KismetMathLibrary.Dot_VectorVector` _velocity _returnvalue_3) 0.0) (`NavMovementComponent.IsFalling` _charactermovement))
      (set `MovementComponent.Velocity` (+ (`KismetMathLibrary.ProjectVectorOnToPlane` _velocity (/ _returnvalue_3 (`KismetMathLibrary.VSize` _returnvalue_3))) (0.0 0.0 0.0)) (`self.CharacterMovement`)))))

(fn `UserConstructionScript`)