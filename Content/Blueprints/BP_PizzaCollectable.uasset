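; BP_PizzaCollectable is a pizza pickup that Spiderman collects by overlapping its box.
; The overlap passes through a DoOnce, casts to BP_Spiderman, then notifies BP_SpidermanGameMode, hides the pizza and plays the Pizza_time sound.
; The Enable event shows the pizza again and resets the DoOnce, so the same actor can be collected again.
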(event `Enable`
  (`SceneComponent.SetVisibility` (`self.Pizza`) true true)
  (goto _label :!via `Reset`))

(event `self.Box.OnComponentBeginOverlap`
  (params (OverlappedComponent :type "PrimitiveComponent Object Reference") (OtherActor :type "Actor Object Reference") (OtherComp :type "PrimitiveComponent Object Reference") (OtherBodyIndex :type Integer) (bFromSweep :type Boolean) (SweepResult :type "HitResult Structure (by ref)"))
  (`/Engine/EditorBlueprintResources/StandardMacros.DoOnce` false :!label _label
    (:`Completed`
      (cast `/Game/Blueprints/BP_Spiderman` OtherActor)
      (bind _asbp_spiderman_game_mode (cast `/Game/Blueprints/BP_SpidermanGameMode` (`GameplayStatics.GetGameMode`)))
      (`/Game/Blueprints/BP_SpidermanGameMode.PizzaCollected` _asbp_spiderman_game_mode)
      (`SceneComponent.SetVisibility` (`self.Pizza`) false true)
      (`GameplayStatics.PlaySound2D` "/Game/Audio/Raw/pizza_time.pizza_time" 1.0 1.0 0.0 null null))))

(fn `UserConstructionScript`)