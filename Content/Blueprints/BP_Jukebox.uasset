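; BP_Jukebox is an interactable jukebox that changes the game's music when Spiderman is near it.
; It enables its own input from player zero on BeginPlay and listens for the E key.
; On press, it checks whether a BP_Spiderman overlaps its Box volume, then calls CycleMusic on BP_SpidermanGameMode, which handles the music change.
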(event `self.ReceiveBeginPlay`
  (`self.EnableInput` (`GameplayStatics.GetPlayerController` 0)))

(event `Key|E`
  (params (Key :type "Key Structure"))
  (:`Pressed`
    (if (> (`KismetArrayLibrary.Array_Length` (`PrimitiveComponent.GetOverlappingActors` (`self.Box`) "/Game/Blueprints/BP_Spiderman.BP_Spiderman_C")) 0)
      (bind _asbp_spiderman_game_mode (cast `/Game/Blueprints/BP_SpidermanGameMode` (`GameplayStatics.GetGameMode`)))
      (`/Game/Blueprints/BP_SpidermanGameMode.CycleMusic` _asbp_spiderman_game_mode))))

(fn `UserConstructionScript`)